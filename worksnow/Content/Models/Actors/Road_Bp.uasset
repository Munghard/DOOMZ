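; Road actor Blueprint that builds a segmented mesh along a spline in the construction script.
; It divides the spline length evenly by the segment count and adds one spline mesh component per segment, placed between consecutive local-space distances.
; Tangents come from normalized spline positions, not spline directions, scaled to segment length.
; The event graph holds only disabled placeholder events, so there is no runtime logic.
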(event EventBeginPlay)

(event Collision|EventActorBeginOverlap
  (params (OtherActor :type Actor%20Object%20Reference)))

(event EventTick
  (params (DeltaSeconds :type Float%20%28single-precision%29)))

(fn ConstructionScript
  (bind _spline (Variables|Default|GetSpline))
  (Variables|Default|SetLenghtPerMesh (/ (Spline|GetSplineLength _spline) (Math|Conversions|ToFloat(Integer) (Variables|Default|GetSegments))))
  (for _index (range 0 (- (Variables|Default|GetSegments) 1))
    (Variables|Default|SetIndex _index)
    (bind _returnvalue (AddComponent|AddSplineMeshComponent false))
    (SplineMesh|SetStartandEnd _returnvalue (Spline|GetLocationatDistanceAlongSpline _spline (* (Variables|Default|GetIndex) (Variables|Default|GetLenghtPerMesh)) "Local") (* (Math|Vector|Normalize (Spline|GetLocationatDistanceAlongSpline _spline (* (Variables|Default|GetIndex) (Variables|Default|GetLenghtPerMesh)) "Local")) (Variables|Default|GetLenghtPerMesh)) (Spline|GetLocationatDistanceAlongSpline _spline (* (+ (Variables|Default|GetIndex) 1) (Variables|Default|GetLenghtPerMesh)) "Local") (* (Math|Vector|Normalize (Spline|GetLocationatDistanceAlongSpline _spline (* (+ (Variables|Default|GetIndex) 1) (Variables|Default|GetLenghtPerMesh)) "Local")) (Variables|Default|GetLenghtPerMesh)) true :!class /Script/Engine.SplineMeshComponent)))