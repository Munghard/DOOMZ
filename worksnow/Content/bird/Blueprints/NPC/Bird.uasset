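; Bird NPC that flies around until a FirstPersonProjectile hits its Sphere component.
; Each tick while alive, it moves without sweep against its right vector by a random Speed-bounded amount and adds a small random yaw.
; The yaw direction tests the negated random speed, so it normally turns negative.
; A projectile hit sets Dead, spawns an explosion and enables physics simulation on Root.
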(event OnComponentHit(Sphere)
  (params (HitComponent :type Primitive%20Component%20Object%20Reference) (OtherActor :type Actor%20Object%20Reference) (OtherComp :type Primitive%20Component%20Object%20Reference) (NormalImpulse :type Vector :default "0, 0, 0") (Hit :type Hit%20Result%20Structure%20%28by%20ref%29))
  (Utilities|Casting|CastToFirstPersonProjectile OtherActor)
  (Variables|Default|SetDead true)
  (Effects|SpawnEmitteratLocation "/Game/StarterContent/Particles/P_Explosion.P_Explosion" (Transformation|GetActorLocation))
  (Physics|SetSimulatePhysics (Variables|Default|Getroot) true))

(event EventBeginPlay
  (Variables|Default|SetOrigin (.location (Transformation|GetActorTransform))))

(event EventTick
  (params (DeltaSeconds :type Float%20%28single-precision%29))
  (bind _speed (Variables|Default|GetSpeed))
  (bind _returnvalue (Math|Random|RandomFloatinRange 5.0 _speed))
  (bind _returnvalue_2 (* _returnvalue -1.0))
  (if (not (Variables|Default|GetDead))
    (Transformation|AddActorWorldOffset (* (Transformation|GetActorRightVector) _returnvalue_2))
    (Class|Actor|AddActorWorldRotation (Math|Rotator|MakeRotator 0.0 0.0 (select (> _returnvalue_2 2.0) (Math|Random|RandomFloatinRange 0.1 0.4) (Math|Random|RandomFloatinRange -0.4 -0.1))))))

(fn ConstructionScript)