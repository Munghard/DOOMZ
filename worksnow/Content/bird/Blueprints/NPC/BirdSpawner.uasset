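; BirdSpawner is an actor that populates the level with up to 100 Bird actors, spawned gradually.
; Tick runs through a randomized Delay and a DoN node, staggering spawns at irregular intervals until the cap is reached.
; Each pass picks a point offset from the spawner by up to SpawnRadius along each positive axis, forming a box rather than a sphere.
; SpawnBirds then always spawns a randomly scaled Bird there, ignoring collisions.
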(event EventTick
  (params (DeltaSeconds :type Float%20%28single-precision%29))
  (bind _self self)
  (bind _spawnradius (Variables|Default|GetSpawnRadius))
  (bind _returnvalue (Transformation|GetActorTransform _self))
  (bind _returnvalue_2 (Math|Random|RandomFloatinRange 0.0 _spawnradius))
  (Utilities|FlowControl|Delay (Math|Random|RandomFloatinRange 0.1 1.0))
  (Utilities|FlowControl|DoN 100
    (:Exit
      (Variables|Default|SetRandomLoc (Math|Vector|MakeVector (+ (.x (.location _returnvalue)) _returnvalue_2) (+ (.y (.location _returnvalue)) _returnvalue_2) (+ (.z (.location _returnvalue)) _returnvalue_2)))
      (CallFunction|SpawnBirds))))

(fn ConstructionScript)

(fn SpawnBirds
  (Game|SpawnActorfromClass "/Game/bird/Blueprints/NPC/Bird.Bird_C" (Math|Transform|MakeTransform (Variables|Default|GetRandomLoc) "0, 0, 0" (* "1.000000,1.000000,1.000000" (Math|Random|RandomFloatinRange 0.5 1.0))) "AlwaysSpawn" 0 0))