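; Sliding lab door that opens automatically on overlap or through Interact, with optional auto-close on leaving the collision.
; Two timelines act as tickers, stepping DoorPosition a fixed amount per update to slide the mesh along local Y, clamped at both ends.
; Reaching the fully open limit clears the Open flag that Interact checks.
; The construction script applies the starting offset, selected door mesh and two materials for door and jamb.
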(event OnComponentEndOverlap(Collision)
  (params (OverlappedComponent :type Primitive%20Component%20Object%20Reference) (OtherActor :type Actor%20Object%20Reference) (OtherComp :type Primitive%20Component%20Object%20Reference) (OtherBodyIndex :type Integer))
  (if (or (Variables|Default|GetAutoClose) (Variables|Default|GetAutoDoor))
    (Variables|Default|SetOpen false)
    (Utilities|FlowControl|Sequence
      (:then_0
        (Timeline|Timeline_1 Stop
          (:Update
            (Math|Float|CompareFloat (Variables|Default|GetDoorPosition) 9e+01
              (:>
                (Variables|Default|SetDoorPosition 9e+01 :!label _label)
                (Variables|Default|SetOpen false))
              (:==
                (goto _label))
              (:<
                (Variables|Default|SetDoorPosition (+ (Variables|Default|GetDoorPosition) 4.0))
                (Transformation|SetRelativeLocation (Variables|Default|GetLabDoor01) (Math|Vector|MakeVector 0.0 (Variables|Default|GetDoorPosition) 0.0) false false :!label _label_2))))))
      (:then_1
        (Timeline|Timeline_0 PlayFromStart
          (:Update
            (Math|Float|CompareFloat (Variables|Default|GetDoorPosition) 0.0
              (:>
                (Variables|Default|SetDoorPosition (- (Variables|Default|GetDoorPosition) 4.0))
                (goto _label_2))
              (:==
                _)
              (:<
                _))
            (Variables|Default|SetDoorPosition 0.0)))))))

(event OnComponentBeginOverlap(Collision)
  (params (OverlappedComponent :type Primitive%20Component%20Object%20Reference) (OtherActor :type Actor%20Object%20Reference) (OtherComp :type Primitive%20Component%20Object%20Reference) (OtherBodyIndex :type Integer) (bFromSweep :type Boolean) (SweepResult :type Hit%20Result%20Structure%20%28by%20ref%29))
  (if (Variables|Default|GetAutoDoor)
    (Variables|Default|SetOpen true)
    (Utilities|FlowControl|Sequence
      (:then_0
        (Timeline|Timeline_0 Stop
          (:Update
            (Math|Float|CompareFloat (Variables|Default|GetDoorPosition) 0.0
              (:>
                (Variables|Default|SetDoorPosition (- (Variables|Default|GetDoorPosition) 4.0))
                (Transformation|SetRelativeLocation (Variables|Default|GetLabDoor01) (Math|Vector|MakeVector 0.0 (Variables|Default|GetDoorPosition) 0.0) false false :!label _label))
              (:==
                (Variables|Default|SetDoorPosition 0.0 :!label _label_2))
              (:<
                (goto _label_2))))))
      (:then_1
        (Timeline|Timeline_1 PlayFromStart
          (:Update
            (Math|Float|CompareFloat (Variables|Default|GetDoorPosition) 9e+01
              (:>
                _)
              (:==
                _)
              (:<
                (Variables|Default|SetDoorPosition (+ (Variables|Default|GetDoorPosition) 4.0))
                (goto _label)))
            (Variables|Default|SetDoorPosition 9e+01)
            (Variables|Default|SetOpen false)))))))

(event EventInteract
  (params (Action :type Actions_ENUM%20Enum :default "NewEnumerator0") (Component :type Actor%20Component%20Object%20Reference) (Meatman_Ref :type Meat%20Man%20Soft%20Object%20Reference))
  (if (not (Variables|Default|GetAutoDoor))
    (if (Variables|Default|GetOpen)
      (Utilities|FlowControl|Sequence
        (:then_0
          (Timeline|Timeline_1 Stop
            (:Update
              (Math|Float|CompareFloat (Variables|Default|GetDoorPosition) 9e+01
                (:>
                  (Variables|Default|SetDoorPosition 9e+01 :!label _label)
                  (Variables|Default|SetOpen false))
                (:==
                  (goto _label))
                (:<
                  (Variables|Default|SetDoorPosition (+ (Variables|Default|GetDoorPosition) 4.0))
                  (Transformation|SetRelativeLocation (Variables|Default|GetLabDoor01) (Math|Vector|MakeVector 0.0 (Variables|Default|GetDoorPosition) 0.0) false false :!label _label_2))))))
        (:then_1
          (Timeline|Timeline_0 PlayFromStart
            (:Update
              (Math|Float|CompareFloat (Variables|Default|GetDoorPosition) 0.0
                (:>
                  (Variables|Default|SetDoorPosition (- (Variables|Default|GetDoorPosition) 4.0))
                  (goto _label_2))
                (:==
                  _)
                (:<
                  _))
              (Variables|Default|SetDoorPosition 0.0)))))
      (else
        (Utilities|FlowControl|Sequence
          (:then_0
            (Timeline|Timeline_0 Stop))
          (:then_1
            (Timeline|Timeline_1 PlayFromStart)))))))

(fn ConstructionScript
  (bind _labdoor01 (Variables|Default|GetLabDoor01))
  ;[1 1 1] Movement
  (Transformation|AddRelativeLocation _labdoor01 (Math|Vector|MakeVector 0.0 (Variables|Default|GetDoorPosition) 0.0) false false)
  ;[1 1 1] Change Door Mesh
  (switch int (Variables|Default|GetDoor%20Mesh)
    (:Default
      (Components|StaticMesh|SetStaticMesh _labdoor01 "/Game/Models/StaticMeshes/Structures/Doors/SM_LabDoor01.SM_LabDoor01" :!label _label))
    (:0
      (goto _label))
    (:1
      (Components|StaticMesh|SetStaticMesh _labdoor01 "/Game/Models/StaticMeshes/Structures/Doors/SM_LabDoor04.SM_LabDoor04")))
  ;[1 1 1] Materail
  (Rendering|Material|SetMaterial _labdoor01 0 (Variables|Default|GetMaterail1))
  (Rendering|Material|SetMaterial (Variables|Default|GetLabDoorjamb01) 1 (Variables|Default|GetMaterail2)))