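; NormalDoor_Bp is an interactable hinged door that toggles between closed and open by swinging its mesh 110 degrees in yaw.
; Interact plays or reverses the DoorCurve timeline based on Open, which updates from the timeline's direction only when the swing finishes.
; The construction script applies the configurable Mesh and pre-rotates doors that start Open, while InteractUIData is an empty stub.
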(event EventBeginPlay)

(event Collision|EventActorBeginOverlap
  (params (OtherActor :type Actor%20Object%20Reference)))

(event EventTick
  (params (DeltaSeconds :type Float%20%28single-precision%29)))

(event EventInteract
  (params (Action :type Actions_ENUM%20Enum :default "NewEnumerator0") (Component :type Actor%20Component%20Object%20Reference) (Meatman_Ref :type Meat%20Man%20Soft%20Object%20Reference))
  (if (not (Variables|Default|GetOpen))
    (bind (_direction _curve) (Timeline|DoorCurve Play)
      (:Update
        (Transformation|SetRelativeRotation (Variables|Default|GetStaticMesh) (Math|Rotator|MakeRotator 0.0 0.0 (* _curve 1.1e+02)) false false))
      (:Finished
        (Variables|Default|SetOpen (Utilities|Enum|Equal(Enum) _direction "Forward"))))
    (else
      (Timeline|DoorCurve Reverse))))

(fn ConstructionScript
  (bind _staticmesh (Variables|Default|GetStaticMesh))
  (Components|StaticMesh|SetStaticMesh _staticmesh (Variables|Default|GetMesh))
  (if (Variables|Default|GetOpen)
    (Transformation|SetRelativeRotation _staticmesh (Math|Rotator|MakeRotator 0.0 0.0 (* 1.0 1.1e+02)) false false)))

(fn InteractUIData
  (return ""))