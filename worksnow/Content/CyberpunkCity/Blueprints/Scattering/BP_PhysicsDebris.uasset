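; BP_PhysicsDebris is a scatterable debris prop that picks its mesh from the DebrisMeshes array.
; The construction script seeds a random stream with DebrisSeed, first re-rolling that seed when FullyRandom is set, then assigns a mesh to DebrisMesh.
; The stream draw's upper bound is the array length, so it can land one past the last entry.
; The event graph holds no active logic.
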(event EventBeginPlay)

(event Collision|EventActorBeginOverlap
  (params (OtherActor :type Actor%20Object%20Reference)))

(event EventTick
  (params (DeltaSeconds :type Float%20%28single-precision%29)))

(fn ConstructionScript
  (bind _debrismeshes (Variables|Default|GetDebrisMeshes))
  (bind _returnvalue (Utilities|Array|Length _debrismeshes))
  (if (Variables|Default|GetFullyRandom)
    (Variables|Default|SetDebrisSeed (Math|Random|RandomInteger _returnvalue)))
  (Math|Random|SetRandomStreamSeed (Variables|Default|GetRandomStream) (Variables|Default|GetDebrisSeed))
  (Components|StaticMesh|SetStaticMesh (Variables|Default|GetDebrisMesh) (Utilities|Array|Get(acopy) (Variables|Default|GetDebrisMeshes) (Math|Random|RandomIntegerinRangefromStream 0 _returnvalue (Variables|Default|GetRandomStream)))))