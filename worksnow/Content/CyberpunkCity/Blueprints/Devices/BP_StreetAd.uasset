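; Street advertisement device for the cyberpunk city that configures its look in the Construction Script, with no runtime logic.
; An optionally random variation index selects the holo screen texture, frame color and left and right light colors through dynamic material instances and light components.
; When the device is off, the screen goes black and both lights hide.
; The mesh randomly rotates 180 degrees on every construction, even with Random disabled.
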(event EventBeginPlay)

(event Collision|EventActorBeginOverlap
  (params (OtherActor :type Actor%20Object%20Reference)))

(event EventTick
  (params (DeltaSeconds :type Float%20%28single-precision%29)))

(fn ConstructionScript
  (CallFunction|Init))

(fn Init
  (bind _sm_streetad1 (Variables|Default|GetSM_StreetAd1))
  (bind _leftcolor (Variables|Default|GetLeftColor))
  (if (Variables|Default|GetRandom)
    (Variables|Default|SetTextureVariation (Math|Random|RandomInteger (Utilities|Array|Length (Variables|Default|GetHoloTextures)))))
  (bind _returnvalue (Rendering|Material|CreateDynamicMaterialInstance _sm_streetad1 0 (Rendering|Material|GetMaterial _sm_streetad1 0) "None" :!class /Script/Engine.PrimitiveComponent))
  (Variables|Default|SetStreetAdMatInst _returnvalue)
  (bind _returnvalue_2 (Rendering|Material|CreateDynamicMaterialInstance _sm_streetad1 1 (Rendering|Material|GetMaterial _sm_streetad1 1) "None" :!class /Script/Engine.PrimitiveComponent))
  (Variables|Default|SetScreenMatInst _returnvalue_2)
  (if (Variables|Default|GetDeviceOn)
    (Rendering|Material|SetTextureParameterValue (Variables|Default|GetScreenMatInst) "HoloT" (Utilities|Array|Get(acopy) (Variables|Default|GetHoloTextures) (Variables|Default|GetTextureVariation)))
    (Rendering|SetVisibility _leftcolor true false)
    (Rendering|Components|Light|SetLightColor _leftcolor (Utilities|Array|Get(acopy) (Variables|Default|GetLeftLightColor) (Variables|Default|GetTextureVariation)) true)
    (Rendering|Components|Light|SetLightColor (Variables|Default|GetRightColor) (Utilities|Array|Get(acopy) (Variables|Default|GetRightLightColor) (Variables|Default|GetTextureVariation)) true)
    (else
      (Rendering|Material|SetTextureParameterValue (Variables|Default|GetScreenMatInst) "HoloT" "/Engine/EngineResources/Black.Black")
      (Rendering|SetVisibility _leftcolor false false)))
  (Rendering|Material|SetVectorParameterValue (Variables|Default|GetStreetAdMatInst) "PlasticColor1" (Utilities|Array|Get(acopy) (Variables|Default|GetStreetAdFrameColor) (Variables|Default|GetTextureVariation)) :!class /Script/Engine.MaterialInstanceDynamic)
  (Transformation|SetRelativeRotation (Variables|Default|GetSM_StreetAd1) (select (Math|Random|RandomBool) "0,180.000000, 0" "0, 0, 0") false false))