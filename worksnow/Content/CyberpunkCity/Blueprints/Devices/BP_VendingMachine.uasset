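; Vending machine prop for the Cyberpunk City set, configured entirely in the construction script with no active runtime logic.
; Init creates dynamic material instances for body and screen, using one variation index, optionally randomized, to pick the plastic color, hologram texture and matching rect light color.
; When the device is off, the screen texture switches to black and the light is hidden, while the body keeps its variation color.
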(event EventBeginPlay)

(event Collision|EventActorBeginOverlap
  (params (OtherActor :type Actor%20Object%20Reference)))

(event EventTick
  (params (DeltaSeconds :type Float%20%28single-precision%29)))

(fn ConstructionScript
  (CallFunction|Init))

(fn Init
  (bind _sm_vendingmachine1 (Variables|Default|GetSM_VendingMachine1))
  (bind _sm_vendingmachine1_screen (Variables|Default|GetSM_VendingMachine1_Screen))
  (bind _rectlight (Variables|Default|GetRectLight))
  (if (Variables|Default|GetRandom)
    (Variables|Default|SetTextureVariation (Math|Random|RandomInteger (Utilities|Array|Length (Variables|Default|GetHoloTextures)))))
  (bind _returnvalue (Rendering|Material|CreateDynamicMaterialInstance _sm_vendingmachine1 0 (Rendering|Material|GetMaterial _sm_vendingmachine1 0) "None" :!class /Script/Engine.PrimitiveComponent))
  (Variables|Default|SetVendingMachineMatInst _returnvalue)
  (bind _returnvalue_2 (Rendering|Material|CreateDynamicMaterialInstance _sm_vendingmachine1_screen 0 (Rendering|Material|GetMaterial _sm_vendingmachine1_screen 0) "None" :!class /Script/Engine.PrimitiveComponent))
  (Variables|Default|SetScreenMatInst _returnvalue_2)
  (if (Variables|Default|GetDeviceOn)
    (Rendering|Material|SetTextureParameterValue (Variables|Default|GetScreenMatInst) "HoloT" (Utilities|Array|Get(acopy) (Variables|Default|GetHoloTextures) (Variables|Default|GetTextureVariation)))
    (Rendering|SetVisibility _rectlight true false)
    (Rendering|Components|Light|SetLightColor _rectlight (Utilities|Array|Get(acopy) (Variables|Default|GetLightColors) (Variables|Default|GetTextureVariation)) true)
    (else
      (Rendering|Material|SetTextureParameterValue (Variables|Default|GetScreenMatInst) "HoloT" "/Engine/EngineResources/Black.Black")
      (Rendering|SetVisibility _rectlight false false)))
  (Rendering|Material|SetVectorParameterValue (Variables|Default|GetVendingMachineMatInst) "PlasticColor" (Utilities|Array|Get(acopy) (Variables|Default|GetVendingMachineColor) (Variables|Default|GetTextureVariation)) :!class /Script/Engine.MaterialInstanceDynamic))