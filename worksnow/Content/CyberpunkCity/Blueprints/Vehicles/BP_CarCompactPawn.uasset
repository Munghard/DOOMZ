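; Compact car pawn Blueprint that drives steering wheel rotation in the car's animation.
; On BeginPlay it runs the parent logic, then casts the mesh's anim instance to Car_Compact_AnimBP and caches it.
; Each Tick it calls the parent, then copies the pawn's SteeringAngle into that AnimBP if the reference is valid.
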(event EventBeginPlay
  (|CallParentFunction)
  (bind _ascar_compact_anim_bp (Utilities|Casting|CastToCar_Compact_AnimBP (Components|SkeletalMesh|GetAnimInstance (Variables|Character|GetMesh))))
  (Variables|Default|SetAnimBP _ascar_compact_anim_bp))

(event Collision|EventActorBeginOverlap
  (params (OtherActor :type Actor%20Object%20Reference)))

(event EventTick
  (params (DeltaSeconds :type Float%20%28single-precision%29))
  (|CallParentFunction DeltaSeconds)
  ;[1 1 1] Update Steering Wheel Rotation
  (if (Utilities|IsValid (Variables|Default|GetAnimBP))
    (Variables|/Game/CyberpunkCity/Models/Vehicles/Compact/Car_Compact_AnimBP.Car_Compact_AnimBP_C|SetSteeringAngle (Variables|Default|GetAnimBP) (Variables|Default|GetSteeringAngle))))

(fn ConstructionScript
  (|CallParentFunction))