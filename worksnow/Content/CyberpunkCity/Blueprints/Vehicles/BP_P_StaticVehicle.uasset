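; Static vehicle prop for the city that randomizes its paint, rim and interior colors and dirt level in the Construction Script.
; InitCar creates dynamic material instances for the mesh's Body, Wheel and Interior slots, found by name.
; A seeded stream picks the colors and body/wheel dirt; FullyRandom rerolls the seed within the paint array's length.
; Rim and interior picks also use the paint array's length as their index range.
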(event EventBeginPlay)

(event Collision|EventActorBeginOverlap
  (params (OtherActor :type Actor%20Object%20Reference)))

(event EventTick
  (params (DeltaSeconds :type Float%20%28single-precision%29)))

(fn ConstructionScript
  (CallFunction|InitCar))

(fn InitCar
  (bind _randomstream (Variables|Default|GetRandomStream))
  (bind _mesh (Variables|Default|GetMesh))
  (bind _carpaintarray (Variables|Default|GetCarPaintArray))
  (bind _returnvalue (Utilities|Array|Length _carpaintarray))
  (if (Variables|Default|GetFullyRandom)
    (Variables|Default|SetSeed (Math|Random|RandomInteger _returnvalue)))
  (Math|Random|SetRandomStreamSeed (Variables|Default|GetRandomStream) (Variables|Default|GetSeed))
  ;[1 1 1] Create Material Instances
  (for (_array_element _array_index) (Class|MeshComponent|GetMaterialSlotNames _mesh)
    (if (Utilities|Name|Equal(Name) _array_element "Body")
      (bind _returnvalue_2 (Rendering|Material|CreateDynamicMaterialInstance _mesh _array_index (Rendering|Material|GetMaterial _mesh _array_index) "None" :!class /Script/Engine.PrimitiveComponent))
      (Variables|Default|SetBodyMatInst _returnvalue_2)
      (elif (Utilities|Name|Equal(Name) _array_element "Wheel")
        (bind _returnvalue_3 (Rendering|Material|CreateDynamicMaterialInstance _mesh _array_index (Rendering|Material|GetMaterial _mesh _array_index) "None" :!class /Script/Engine.PrimitiveComponent))
        (Variables|Default|SetWheelMatInst _returnvalue_3)
        (elif (Utilities|Name|Equal(Name) _array_element "Interior")
          (bind _returnvalue_4 (Rendering|Material|CreateDynamicMaterialInstance _mesh _array_index (Rendering|Material|GetMaterial _mesh _array_index) "None" :!class /Script/Engine.PrimitiveComponent))
          (Variables|Default|SetInteriorMatInst _returnvalue_4)))))
  ;[1 1 1] Set Colors
  (Rendering|Material|SetVectorParameterValue (Variables|Default|GetBodyMatInst) "CarPaintColor" (Utilities|Array|Get(acopy) (Variables|Default|GetCarPaintArray) (Class|KismetMathLibrary|RandomIntegerfromStream _returnvalue _randomstream)) :!class /Script/Engine.MaterialInstanceDynamic)
  (Rendering|Material|SetVectorParameterValue (Variables|Default|GetWheelMatInst) "RimColor1" (Utilities|Array|Get(acopy) (Variables|Default|GetRimColorArray) (Class|KismetMathLibrary|RandomIntegerfromStream _returnvalue _randomstream)) :!class /Script/Engine.MaterialInstanceDynamic)
  (Rendering|Material|SetVectorParameterValue (Variables|Default|GetInteriorMatInst) "PlasticColor" (Utilities|Array|Get(acopy) (Variables|Default|GetInteriorColorArray) (Class|KismetMathLibrary|RandomIntegerfromStream _returnvalue _randomstream)) :!class /Script/Engine.MaterialInstanceDynamic)
  ;[1 1 1] Set Dirt
  (Rendering|Material|SetScalarParameterValue (Variables|Default|GetBodyMatInst) "DirtBlendingMultiplier" (Math|Random|RandomFloatinRangefromStream 0.0 3.0 (Variables|Default|GetRandomStream)) :!class /Script/Engine.MaterialInstanceDynamic))