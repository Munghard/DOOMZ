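; BP_Skybridge is a spline-based skybridge actor that positions its Start and End pieces in the construction script, with no runtime logic.
; SetStartEndMeshes puts Start at the spline origin, yawed 180 degrees, and End one Spacing step past the last whole interval of spline length.
; Both pieces share the spline start's height and have zero pitch, keeping them level; only Start inherits spline roll.
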(event EventBeginPlay)

(event Collision|EventActorBeginOverlap
  (params (OtherActor :type Actor%20Object%20Reference)))

(event EventTick
  (params (DeltaSeconds :type Float%20%28single-precision%29)))

(fn ConstructionScript
  (|CallParentFunction)
  (CallFunction|SetStartEndMeshes))

(fn SetStartEndMeshes
  (bind _spline (Variables|Default|GetSpline))
  (bind _spline_2 (Variables|Default|GetSpline))
  (bind _spacing (Variables|Default|GetSpacing))
  (bind _returnvalue (Spline|GetSplineLength _spline_2))
  (bind _returnvalue_2 (Spline|GetLocationatDistanceAlongSpline _spline_2 0.0 "World"))
  (bind _returnvalue_3 (* 0 _spacing))
  (bind _returnvalue_4 (Math|Float|Division(WholeandRemainder) _returnvalue _spacing))
  (bind _returnvalue_5 (Spline|GetLocationatDistanceAlongSpline _spline _returnvalue_3 "World"))
  (bind _returnvalue_6 (Spline|GetRotationatDistanceAlongSpline _spline _returnvalue_3 "World"))
  (bind (_roll _pitch _yaw) (Math|Rotator|BreakRotator _returnvalue_6))
  (bind _returnvalue_7 (+ _returnvalue_4 1))
  (bind _returnvalue_8 (* _returnvalue_7 _spacing))
  (bind _returnvalue_9 (Spline|GetLocationatDistanceAlongSpline _spline _returnvalue_8 "World"))
  (Transformation|SetWorldTransform (Variables|Default|GetStart) (Math|Transform|MakeTransform (Math|Vector|MakeVector (.x _returnvalue_5) (.y _returnvalue_5) (.z _returnvalue_2)) (Math|Rotator|MakeRotator _roll 0.0 (+ _yaw 1.8e+02))) false false)
  (Transformation|SetWorldTransform (Variables|Default|GetEnd) (Math|Transform|MakeTransform (Math|Vector|MakeVector (.x _returnvalue_9) (.y _returnvalue_9) (.z _returnvalue_2)) (Math|Rotator|MakeRotator 0.0 0.0 (.Yaw (Math|Rotator|BreakRotator (Spline|GetRotationatDistanceAlongSpline _spline _returnvalue_8 "World"))))) false false))